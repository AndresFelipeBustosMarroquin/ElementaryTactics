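; Space is an actor that holds one creature slot and handles spawning and destroying the creature on it.
; Spawn looks up the creature enum in the Classes map from Instance, spawns that class at its own transform with an Explosion effect, and stores the type and actor.
; A missing class prints an error; Destroy removes the stored actor and resets the creature to empty.
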(fn `Destroy`
  (`self.K2_DestroyActor` (`self.Actor`))
  (set `self.Creature` "NewEnumerator3"))

(fn `Spawn`
  (params (Creature :type "/Game/Enumeration/Creature Enum (by ref)"))
  (bind _instance (`/Game/Blueprints/Function/Library/InstanceTools.Instance`))
  (bind (_value _returnvalue) (`BlueprintMapLibrary.Map_Find` (`/Game/Blueprints/Class/Context/Instance.Classes` _instance) Creature))
  (if _returnvalue
    (bind _returnvalue_2 (`|SpawnActorFromClass` _value (`self.GetTransform`) "Undefined" "MultiplyWithRoot" null null))
    (`/Game/Blueprints/Function/Library/Tools.Spawn System` "/Game/Niagara/System/Explosion.Explosion" (`self.K2_GetActorLocation`))
    (set `self.Creature` Creature)
    (set `self.Actor` _returnvalue_2)
    (else
      (`/Game/Blueprints/Function/Library/Tools.Print` "Space/Spawn: Class not found" true))))

(fn `UserConstructionScript`)