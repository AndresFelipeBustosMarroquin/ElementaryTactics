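; Instance Blueprint that tallies creatures and orbs separately for the player and the enemy.
; Four maps hold counts keyed by type; add functions pick the side's map via IsPlayer, then increment the existing entry or start it at one.
; Creature deletion removes the whole entry rather than decrementing, and getters return maps by side.
; Delete-all functions remove two hard-coded enum keys per map instead of clearing it.
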(fn `Add Creature`
  (params (`Is Player` :type Boolean) (Creature :type "/Game/Enumeration/Creature Enum (by ref)"))
  (if `Is Player`
    (`self.Calculate Creature` (`self.Creatures Player`) Creature)
    (else
      (`self.Calculate Creature` (`self.Creatures Enemy`) Creature))))

(fn `Add Orb`
  (params (`Is Player` :type Boolean) (Orb :type "/Game/Enumeration/Orbs Enum" :default "NewEnumerator8"))
  (if `Is Player`
    (`self.Calculate Orb` (`self.Orbs Player`) Orb)
    (else
      (`self.Calculate Orb` (`self.Orbs Enemy`) Orb))))

(fn `Calculate Creature`
  (params (Creatures :type "Map of /Game/Enumeration/Creature Enum to Integer (by ref)") (Creature :type "/Game/Enumeration/Creature Enum (by ref)"))
  (bind (_value _returnvalue) (`BlueprintMapLibrary.Map_Find` Creatures Creature))
  (if _returnvalue
    (`BlueprintMapLibrary.Map_Add` Creatures Creature (+ _value 1))
    (else
      (`BlueprintMapLibrary.Map_Add` Creatures Creature 1))))

(fn `Calculate Orb`
  (params (Creatures :type "Map of /Game/Enumeration/Orbs Enum to Integer (by ref)") (Orb :type "/Game/Enumeration/Orbs Enum (by ref)"))
  (bind (_value _returnvalue) (`BlueprintMapLibrary.Map_Find` Creatures Orb))
  (if _returnvalue
    (`BlueprintMapLibrary.Map_Add` Creatures Orb (+ _value 1))
    (else
      (`BlueprintMapLibrary.Map_Add` Creatures Orb 1))))

(fn `Delete all Creature`
  (bind _creatures_player (`self.Creatures Player`))
  (bind _creatures_enemy (`self.Creatures Enemy`))
  (`self.Remove Creatures` _creatures_player "NewEnumerator0")
  (`self.Remove Creatures` _creatures_player "NewEnumerator1")
  (`self.Remove Creatures` _creatures_enemy "NewEnumerator0")
  (`self.Remove Creatures` _creatures_enemy "NewEnumerator1"))

(fn `Delete all Orb`
  (bind _orbs_enemy (`self.Orbs Enemy`))
  (bind _orbs_player (`self.Orbs Player`))
  (`BlueprintMapLibrary.Map_Remove` _orbs_enemy "NewEnumerator7")
  (`BlueprintMapLibrary.Map_Remove` _orbs_player "NewEnumerator7")
  (`BlueprintMapLibrary.Map_Remove` _orbs_player "NewEnumerator6")
  (`BlueprintMapLibrary.Map_Remove` _orbs_enemy "NewEnumerator6"))

(fn `Delete Creatures`
  (params (`Is Player` :type Boolean) (Creature :type "/Game/Enumeration/Creature Enum" :default "NewEnumerator3"))
  (if `Is Player`
    (`self.Remove Creatures` (`self.Creatures Player`) Creature)
    (else
      (`self.Remove Creatures` (`self.Creatures Enemy`) Creature))))

(fn `Get Creatures`
  (params (`Is Player` :type Boolean))
  (returns (Creatures :type "Map of /Game/Enumeration/Creature Enum to Integer"))
  (if `Is Player`
    (return (`self.Creatures Player`))
    (else
      (return (`self.Creatures Enemy`)))))

(fn `Get Orbs`
  (params (`Is Player` :type Boolean))
  (returns (Orbs :type "Map of /Game/Enumeration/Orbs Enum to Integer"))
  (if `Is Player`
    (return (`self.Orbs Player`))
    (else
      (return (`self.Orbs Enemy`)))))

(fn `Remove Creatures`
  (params (Creatures :type "Map of /Game/Enumeration/Creature Enum to Integer (by ref)") (Creature :type "/Game/Enumeration/Creature Enum" :default "NewEnumerator3"))
  (`BlueprintMapLibrary.Map_Remove` Creatures Creature))